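; Player controller that moves the player character along world X/Y and adds a double-tap dash for BP_Ro3ot.
; Looping timers poll hardcoded ZQSD key presses and periodically clear per-axis press counters, which Tick increments.
; Axis events add movement input until a counter reaches two, then, only if IsAgressif is set, launch the character with a brief invulnerability window.
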(event `self.ReceiveBeginPlay`
  (`KismetSystemLibrary.K2_SetTimerDelegate` (delegate `ResetPresses`) 0.3 true)
  (`KismetSystemLibrary.K2_SetTimerDelegate` (delegate `CHI`) 0.01 true)
  (`KismetSystemLibrary.K2_SetTimerDelegate` (delegate `CVI`) 0.01 true))

(event `ResetPresses`
  (if (not (`self.HIs Pressed`))
    (set `self.pressesH` 0)
    (if (not (`self.VIs Pressed`))
      (set `self.pressesV` 0))))

(event `CHI`
  (bind _ispressed (`self.CheckHorizontalInputs`))
  (set `self.HIs Pressed` _ispressed))

(event `CVI`
  (bind _ispressed (`self.CheckVerticalInputs`))
  (set `self.VIs Pressed` _ispressed))

(event `self.ReceiveTick`
  (params (DeltaSeconds :type "Float (single-precision)"))
  (bind _pressesh (`self.pressesH`))
  (bind _pressesv (`self.pressesV`))
  ;[1 1 1] DashManagement
  (if (`self.HIs Pressed`)
    (`/Engine/EditorBlueprintResources/StandardMacros.DoOnce` false :!label _label
      (:`Completed`
        (if (< _pressesh 2)
          (`/Engine/EditorBlueprintResources/StandardMacros.IncrementInt` _pressesh
            (:`  `
              (goto _label :!via `Reset`))))))
    (elif (`self.VIs Pressed`)
      (`/Engine/EditorBlueprintResources/StandardMacros.DoOnce` false :!label _label_2
        (:`Completed`
          (if (< _pressesv 2)
            (`/Engine/EditorBlueprintResources/StandardMacros.IncrementInt` _pressesv
              (:`  `
                (goto _label_2 :!via `Reset`)))))))))

(event `InputAxis|Horizontal`
  (params (AxisValue :type "Float (single-precision)"))
  (bind _returnvalue (`GameplayStatics.GetPlayerCharacter` 0))
  ;[1 1 1] Horizontal Movement - Dash
  (bind _output_get (set `self.Axis Value` AxisValue))
  (if (or (> _output_get 0.0) (< _output_get 0.0))
    (if (>= (`self.pressesH`) 2)
      (bind _asbp_ro_3ot (cast `/Game/Blueprint/Ro3ot/BP_Ro3ot` _returnvalue))
      (if (`/Game/Blueprint/Ro3ot/BP_Ro3ot.isAgressif` _asbp_ro_3ot)
        (set `PlayerCube.invulnerabiltyFrame` true _asbp_ro_3ot)
        (`Character.LaunchCharacter` _asbp_ro_3ot (+ (`KismetMathLibrary.MakeVector` 0.0 (* (`self.Axis Value`) 4250.0)) (0.0 0.0 0.0)) false false)
        (`KismetSystemLibrary.Delay` 0.5)
        (set `PlayerCube.invulnerabiltyFrame` false _asbp_ro_3ot))
      (else
        (`Pawn.AddMovementInput` _returnvalue (0.0 200.0 0.0) (`self.Axis Value`) false)))))

(event `InputAxis|Vertical`
  (params (AxisValue :type "Float (single-precision)"))
  (bind _returnvalue (`GameplayStatics.GetPlayerCharacter` 0))
  ;[1 1 1] Vertical Movement - Dash
  (bind _output_get (set `self.Axis Value` AxisValue))
  (if (or (> _output_get 0.0) (< _output_get 0.0))
    (if (>= (`self.pressesV`) 2)
      (bind _asbp_ro_3ot (cast `/Game/Blueprint/Ro3ot/BP_Ro3ot` _returnvalue))
      (if (`/Game/Blueprint/Ro3ot/BP_Ro3ot.isAgressif` _asbp_ro_3ot)
        (set `PlayerCube.invulnerabiltyFrame` true _asbp_ro_3ot)
        (`Character.LaunchCharacter` _asbp_ro_3ot (+ (`KismetMathLibrary.MakeVector` (* (`self.Axis Value`) 4250.0)) (0.0 0.0 0.0)) false false)
        (`KismetSystemLibrary.Delay` 0.5)
        (set `PlayerCube.invulnerabiltyFrame` false _asbp_ro_3ot))
      (else
        (`Pawn.AddMovementInput` _returnvalue (200.0 0.0 0.0) (`self.Axis Value`) false)))))

(fn `CheckHorizontalInputs`
  (returns (isPressed :type Boolean))
  (return (or (`self.WasInputKeyJustPressed` self "Q") (`self.WasInputKeyJustPressed` self "D"))))

(fn `CheckVerticalInputs`
  (returns (isPressed :type Boolean))
  (return (or (`self.WasInputKeyJustPressed` self "Z") (`self.WasInputKeyJustPressed` self "S"))))

(fn `UserConstructionScript`)