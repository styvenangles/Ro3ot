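; BP_Ro3ot is the player's robot character, which creates the HUD, turns toward the cursor and opens a pause menu on P.
; Tick yaws the capsule to the cursor hit point and polls HP, starting an invulnerability window on any change.
; That window blinks a translucent dynamic material for about a second, then restores the base one.
; SaveRo3ot applies HP and a walk-speed multiplier from an indexed value array.
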(event `self.ReceiveBeginPlay`
  (bind _returnvalue (`|CreateWidget` "/Game/UI/Player/BP_HUD.BP_HUD_C" (`GameplayStatics.GetPlayerController` 0)))
  (bind _output_get (set `self.HUD` _returnvalue))
  (`UserWidget.AddToViewport` _output_get 0)
  (set `PlayerController.bShowMouseCursor` false (`GameplayStatics.GetPlayerController` 0))
  (bind _returnvalue_2 (`self.GetHp`))
  (bind _output_get_2 (set `self.RoBotMaxHp` _returnvalue_2))
  (bind _output_get_3 (set `self.RoBotHp` _output_get_2))
  (set `self.RoBotLastHp` _output_get_3))

(event `Key|P`
  (params (Key :type "Key Structure"))
  (bind _returnvalue (`GameplayStatics.GetPlayerController` 0))
  (:`Pressed`
    (bind _returnvalue_2 (`|CreateWidget` "/Game/UI/Pause.Pause_C" (`GameplayStatics.GetPlayerController` 0)))
    (`UserWidget.AddToViewport` _returnvalue_2 0)
    (`WidgetBlueprintLibrary.SetInputMode_UIOnlyEx` _returnvalue _returnvalue_2)
    (set `PlayerController.bShowMouseCursor` true _returnvalue)
    (`GameplayStatics.SetGamePaused` true)))

(event `self.ReceiveTick`
  (params (DeltaSeconds :type "Float (single-precision)"))
  (bind (_returnvalue_roll _returnvalue_pitch) (`KismetMathLibrary.BreakRotator` (`self.K2_GetActorRotation`)))
  (bind (_returnvalue_roll_2 _returnvalue_pitch_2 _returnvalue_yaw) (`KismetMathLibrary.BreakRotator` (`KismetMathLibrary.FindLookAtRotation` (`self.K2_GetActorLocation`) (`.Location` (`GameplayStatics.BreakHitResult` (`PlayerController.GetHitResultUnderCursorByChannel` (`GameplayStatics.GetPlayerController` 0) "TraceTypeQuery1" true))))))
  (`SceneComponent.K2_SetWorldRotation` (`self.CapsuleComponent`) (`KismetMathLibrary.MakeRotator` _returnvalue_roll _returnvalue_pitch _returnvalue_yaw) false false)
  (bind _returnvalue (`self.GetHp`))
  (set `self.RoBotHp` _returnvalue)
  (if (!= (`self.RoBotHp`) (`self.RoBotLastHp`))
    (`self.SetInvulnerabiltyFrame`)
    (set `self.RoBotLastHp` (`self.RoBotHp`))))

(event `SetInvulnerabiltyFrame`
  (bind _robottransmatinst (`self.RobotTransMatInst`))
  (set `self.invulnerabiltyFrame` true)
  (`PrimitiveComponent.SetMaterial` (`self.Mesh`) 0 _robottransmatinst)
  (`MaterialInstanceDynamic.SetScalarParameterValue` _robottransmatinst "OpacityControl" 0.0)
  (`KismetSystemLibrary.Delay` 0.25)
  (`MaterialInstanceDynamic.SetScalarParameterValue` _robottransmatinst "OpacityControl" 1.0)
  (`KismetSystemLibrary.Delay` 0.25)
  (`MaterialInstanceDynamic.SetScalarParameterValue` _robottransmatinst "OpacityControl" 0.0)
  (`KismetSystemLibrary.Delay` 0.25)
  (`MaterialInstanceDynamic.SetScalarParameterValue` _robottransmatinst "OpacityControl" 1.0)
  (`KismetSystemLibrary.Delay` 0.25)
  (`PrimitiveComponent.SetMaterial` (`self.Mesh`) 0 (`self.RobotBaseMatInst`))
  (set `self.invulnerabiltyFrame` false))

(event `SaveRo3ot`
  (params (ValueEntries :type "Array of String"))
  (bind _charactermovement (`self.CharacterMovement`))
  (for (_array_element _array_index) ValueEntries
    (switch `int` _array_index
      (:`0`
        (set `self.RoBotHp` (`KismetStringLibrary.Conv_StringToInt` _array_element)))
      (:`4`
        (bind _output_get (set `self.Mouvement Speed` (`KismetStringLibrary.Conv_StringToDouble` _array_element)))
        (set `CharacterMovementComponent.MaxWalkSpeed` (* _output_get (`CharacterMovementComponent.MaxWalkSpeed` _charactermovement)) _charactermovement)))))

(fn `UserConstructionScript`
  (`/Engine/EditorBlueprintResources/StandardMacros.FlipFlop`
    (:`A`
      (bind _returnvalue (`KismetMaterialLibrary.CreateDynamicMaterialInstance` "/Game/Blueprint/Ro3ot/Rig/Robot_Gentil_Inst.Robot_Gentil_Inst"))
      (set `self.RobotBaseMatInst` _returnvalue)
      (bind _returnvalue_2 (`KismetMaterialLibrary.CreateDynamicMaterialInstance` "/Game/Blueprint/Ro3ot/Rig/Robot_Gentil_Translucent_Inst.Robot_Gentil_Translucent_Inst"))
      (set `self.RobotTransMatInst` _returnvalue_2))
    (:`B`
      (`PrimitiveComponent.SetMaterial` (`self.Mesh`) 0 (`self.RobotBaseMatInst`)))))