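; BP_EnemyRed is the red robot enemy Blueprint.
; On BeginPlay it sets its scrap to a random amount within a small range, and on every Tick it calls Shoot while IsShooting is true.
; The construction script creates a dynamic instance of the red robot material, stores it in RedMatInst and applies it to the mesh.
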(event `self.ReceiveBeginPlay`
  (`self.SetScrap` (`KismetMathLibrary.RandomFloatInRange` 5.0 9.0)))

(event `self.ReceiveTick`
  (params (DeltaSeconds :type "Float (single-precision)"))
  (if (`self.Is Shooting`)
    (`self.Shoot` self)))

(fn `UserConstructionScript`
  (bind _returnvalue (`KismetMaterialLibrary.CreateDynamicMaterialInstance` "/Game/Blueprint/Enemies/Rig/Robot_Mechant_Red_Inst.Robot_Mechant_Red_Inst"))
  (bind _output_get (set `self.RedMatInst` _returnvalue))
  (`PrimitiveComponent.SetMaterial` (`self.Mesh`) 0 _output_get))