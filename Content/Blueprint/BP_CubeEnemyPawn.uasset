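; Cube enemy pawn that turns to face the player and fires on a repeating timer.
; BeginPlay starts LoopShoot, which calls Shoot and re-sets a one-second looping timer on itself each time it runs.
; Tick rotates the whole actor toward the first player's pawn using a look-at from the mesh, and prints the ProjectileLocation world position as debug output.
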(event `self.ReceiveBeginPlay`
  (`self.LoopShoot`))

(event `LoopShoot`
  (`KismetSystemLibrary.K2_SetTimerDelegate` (delegate `LoopShoot`) 1.0 true)
  (`self.Shoot`))

(event `self.ReceiveTick`
  (params (DeltaSeconds :type "Float (single-precision)"))
  (`self.K2_SetActorRotation` (`KismetMathLibrary.FindLookAtRotation` (`SceneComponent.K2_GetComponentLocation` (`self.Mesh`)) (`self.K2_GetActorLocation` (`GameplayStatics.GetPlayerPawn` 0))))
  (`KismetSystemLibrary.PrintString` (`KismetStringLibrary.Conv_VectorToString` (`SceneComponent.K2_GetComponentLocation` (`self.ProjectileLocation`)))))

(fn `UserConstructionScript`)