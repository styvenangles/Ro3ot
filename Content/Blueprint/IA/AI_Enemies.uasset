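; AI controller for enemies that runs the BT_Enemies behavior tree and feeds it perception of the player.
; Fresh AI Perception stimuli that sense a PlayerCube set the in-range flag and store that actor and its current location in the blackboard.
; A fresh lost stimulus from any actor clears only the flag, leaving the stored actor and location in place.
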(event `self.ReceiveBeginPlay`
  (`self.RunBehaviorTree` "/Game/Blueprint/IA/BT_Enemies.BT_Enemies"))

(event `self.ReceiveTick`
  (params (DeltaSeconds :type "Float (single-precision)")))

(event `self.AIPerception.OnTargetPerceptionUpdated`
  (params (Actor :type "Actor Object Reference") (Stimulus :type "AIStimulus Structure"))
  (bind (_age _expirationage _strength _stimuluslocation _receiverlocation _tag _bsuccessfullysensed) (break `AIStimulus` Stimulus))
  (bind _blackboardenemies (`self.BlackboardEnemies`))
  (if (< _age 1.0)
    (if _bsuccessfullysensed
      (bind _asplayer_cube (cast `PlayerCube` Actor))
      (`BlackboardComponent.SetValueAsBool` _blackboardenemies "isInRange" _bsuccessfullysensed)
      (`BlackboardComponent.SetValueAsObject` _blackboardenemies "EnemyActor" _asplayer_cube)
      (`BlackboardComponent.SetValueAsVector` _blackboardenemies "EnemyLocation" (`self.K2_GetActorLocation` _asplayer_cube))
      (else
        (`BlackboardComponent.SetValueAsBool` (`self.BlackboardEnemies`) "isInRange" false)))))

(fn `UserConstructionScript`)