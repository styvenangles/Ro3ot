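; Behavior tree task that stops yellow, orange or red enemies shooting and picks a location offset from the player, BP_Ro3ot.
; It switches on the pawn's class display name to clear IsShooting, then all three branches share the location logic.
; The target is the player's position minus the unit enemy-to-player direction and a fixed world X/Y offset.
; It debug-prints that vector, writes it to the blackboard key and finishes successfully.
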(event `self.ReceiveExecuteAI`
  (params (OwnerController :type "AIController Object Reference") (ControlledPawn :type "Pawn Object Reference"))
  (switch `string` (`KismetSystemLibrary.GetClassDisplayName` (`GameplayStatics.GetObjectClass` ControlledPawn))
    (:`BP_EnemyYellow_C`
      (bind _asbp_enemy_yellow (cast `/Game/Blueprint/Enemies/BP_EnemyYellow` ControlledPawn))
      (set `/Game/Blueprint/Enemies/BP_EnemyYellow.Is Shooting` false _asbp_enemy_yellow))
    (:`BP_EnemyOrange_C`
      (bind _asbp_enemy_orange (cast `/Game/Blueprint/Enemies/BP_EnemyOrange` ControlledPawn))
      (set `/Game/Blueprint/Enemies/BP_EnemyOrange.Is Shooting` false _asbp_enemy_orange))
    (:`BP_EnemyRed_C`
      (bind _asbp_enemy_red (cast `/Game/Blueprint/Enemies/BP_EnemyRed` ControlledPawn))
      (set `/Game/Blueprint/Enemies/BP_EnemyRed.Is Shooting` false _asbp_enemy_red)))
  (bind _asbp_ro_3ot (cast `/Game/Blueprint/Ro3ot/BP_Ro3ot` (`GameplayStatics.GetPlayerCharacter` 0)))
  (bind _returnvalue (`SceneComponent.K2_GetComponentLocation` (`Actor.RootComponent` _asbp_ro_3ot)))
  (bind _returnvalue_2 (- _returnvalue (`KismetMathLibrary.GetDirectionUnitVector` (`Actor.K2_GetActorLocation` ControlledPawn) _returnvalue) (250.0 250.0 0.0)))
  (`KismetSystemLibrary.PrintString` (`KismetStringLibrary.Conv_VectorToString` _returnvalue_2))
  (`BTFunctionLibrary.SetBlackboardValueAsVector` (`self.Key`) _returnvalue_2)
  (`self.FinishExecute` true))