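; Wave manager that runs numbered enemy waves, starting each after a short printed countdown on a looping timer.
; Each wave reads the DataTable row named by WaveNumber and spawns every entry's enemy class and count at its spawn point.
; A one-second Delay loop polls spawned enemies for validity, advancing the wave when none remain.
; A missing row means victory, showing the Victory widget and pausing the game.
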(event `self.ReceiveBeginPlay`
  (`self.Check Enemy Remaining`))

(event `Check Enemy Remaining`
  (bind _returnvalue (`KismetSystemLibrary.K2_SetTimerDelegate` (delegate `Count`) 1.0 true))
  (set `self.Timer` 3))

(event `Count`
  (`KismetSystemLibrary.PrintString` (`KismetStringLibrary.Conv_IntToString` (`self.Timer`)))
  (`/Engine/EditorBlueprintResources/StandardMacros.DecrementInt` (`self.Timer`)
    (:`  `
      (if (== (`self.Timer`) 0)
        (`KismetSystemLibrary.K2_ClearAndInvalidateTimerHandle` (stale `Check Enemy Remaining` _returnvalue))
        (`self.Begin Wave`)))))

(event `Begin Wave`
  (bind _returnvalue (`|GetDataTableRow` (`self.Data Table`) (`KismetStringLibrary.Conv_StringToName` (`KismetStringLibrary.Conv_IntToString` (`self.Wave Number`))))
    (:`then`
      (for _array_element (`.EnemyInfos_3_CCDBB8A34AA6F99637DAD082D14BE017` (break `/Game/Blueprint/EnemyWave/WaveInfo` _returnvalue))
        (`self.SpawnEnemy` _array_element))
      (`self.CheckIfEnemyDead`))
    (:`RowNotFound`
      (`KismetSystemLibrary.PrintString` "Row Empty")
      (`self.Victory`))))

(event `CheckIfEnemyDead`
  (bind _output_get (`self.CheckIfEnemiesAllDead` :!label _label))
  (if _output_get
    (`KismetSystemLibrary.PrintString` "All Enemies Dead")
    (`/Engine/EditorBlueprintResources/StandardMacros.IncrementInt` (`self.Wave Number`)
      (:`  `
        (`self.Check Enemy Remaining`)))
    (else
      (`KismetSystemLibrary.Delay` 1.0)
      (goto _label))))

(fn `CheckIfEnemiesAllDead`
  (returns (Output_Get :type Boolean))
  (locals (Dead :type Boolean :default true))
  (for _array_element (`self.Current Enemies`)
    (`/Engine/EditorBlueprintResources/StandardMacros.IsValid` _array_element
      (:`Is Valid`
        (set `local.Dead` false))))
  (return (`local.Dead`)))

(fn `SpawnEnemy`
  (params (EnemyInfo :type "/Game/Blueprint/EnemyWave/EnemyInfo Structure (by ref)"))
  (locals (`Current Spawn Point` :type "Array of /Game/Blueprint/EnemyWave/WaveGenerator Object Reference") (EnemyRef :type "/Game/Blueprint/EnemyWave/EnemyInfo Structure"))
  (bind _enemyref_enemyclass (break `/Game/Blueprint/EnemyWave/EnemyInfo` (`local.EnemyRef`)))
  (bind (_enemyref_enemyclass_2 _enemyref_enemynumber) (break `/Game/Blueprint/EnemyWave/EnemyInfo` (`local.EnemyRef`)))
  (bind _output_get (set `local.EnemyRef` EnemyInfo))
  (for _ (range 1 (+ _enemyref_enemynumber 1))
    (bind _returnvalue (`|SpawnActorFromClass` _enemyref_enemyclass (`self.GetTransform` (`|ConvertAsset` (`.SpawnPoint_14_29FA1C504CFFEF9F1A339493E74AC465` (break `/Game/Blueprint/EnemyWave/EnemyInfo` _output_get)))) "AdjustIfPossibleButAlwaysSpawn" "OverrideRootScale" null null))
    (`KismetArrayLibrary.Array_Add` (`self.Current Enemies`) _returnvalue)))

(fn `UserConstructionScript`)

(fn `Victory`
  (bind _returnvalue (`GameplayStatics.GetPlayerController` 0))
  (bind _returnvalue_2 (`|CreateWidget` "/Game/UI/Victory.Victory_C" _returnvalue))
  (`UserWidget.AddToViewport` _returnvalue_2 0)
  (`WidgetBlueprintLibrary.SetInputMode_UIOnlyEx` _returnvalue (`/Game/UI/Victory.Replay_Button` _returnvalue_2))
  (`GameplayStatics.SetGamePaused` true))