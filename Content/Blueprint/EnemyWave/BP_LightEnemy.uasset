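; BP_LightEnemy is a wave enemy that chases the player's pawn and carries an HP bar.
; Shortly after BeginPlay it targets the player's pawn, then Tick drives a delayed AI MoveTo until it is flagged in attack range.
; Range and attack events, not called here, check the Player tag and damage the third-person character by class name.
; Tick also refreshes the life-bar widget from current and max HP.
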(event `self.ReceiveBeginPlay`
  (bind _returnvalue (`GameplayStatics.GetPlayerController` 0))
  (bind _returnvalue_2 (`Controller.K2_GetPawn` _returnvalue))
  (`KismetSystemLibrary.Delay` 1.0)
  (if (!= _returnvalue null)
    (`self.TargetEnemy` _returnvalue_2 (`self.K2_GetActorLocation` _returnvalue_2))))

(event `self.ReceiveTick`
  (params (DeltaSeconds :type "Float (single-precision)"))
  (bind _targetactor (`self.targetActor`))
  (`self.setPercentage`)
  (if (!= _targetactor null)
    (if (not (`self.isInRangeToAttack`))
      (`self.MoveToPlayer` _targetactor (`self.Enemy Location`)))))

(event `self.TargetEnemy`
  (params (Enemy :type "Actor Object Reference") (Location :type "Vector Structure") (isPlayer :type Boolean))
  (set `self.targetActor` Enemy)
  (set `self.Enemy Location` Location))

(event `self.InRangeEnemy`
  (params (Enemy :type "Actor Object Reference") (isPlayer :type Boolean))
  (if (`self.ActorHasTag` Enemy "Player")
    (set `self.isInRangeToAttack` true)
    (else
      (set `self.isInRangeToAttack` false))))

(event `self.AttackEnemy`
  (params (Enemy :type "Actor Object Reference") (Damage :type "Float (single-precision)") (isPlayer :type Boolean))
  (if (!= null Enemy)
    (switch `string` (`KismetSystemLibrary.GetClassDisplayName` (`GameplayStatics.GetObjectClass` Enemy))
      (:`BP_ThirdPersonCharacter_C`
        (bind _asbp_third_person_character (cast `/Game/ThirdPerson/Blueprints/BP_ThirdPersonCharacter` Enemy))
        (`Ro3otCharacter.takeDamage` _asbp_third_person_character (`KismetMathLibrary.FTrunc` (`self.AttackDamage`)))))))

(event `MoveToPlayer`
  (params (Enemy :type "Actor Object Reference") (EnemyLocation :type "Vector Structure"))
  (`KismetSystemLibrary.Delay` 0.5)
  (`|AIMoveTo` self EnemyLocation Enemy 5.0 true))

(event `setPercentage`
  (bind _asw_life_bar (cast `/Game/UI/Enemy/W_LifeBar` (`WidgetComponent.GetUserWidgetObject` (`self.LifeBar`))))
  (`ProgressBar.SetPercent` (`/Game/UI/Enemy/W_LifeBar.ProgressBar_43` _asw_life_bar) (/ (`KismetMathLibrary.Conv_IntToDouble` (`self.Hp`)) (`KismetMathLibrary.Conv_IntToDouble` (`self.MaxHp`))))
  (`TextBlock.SetText` (`/Game/UI/Enemy/W_LifeBar.HpEnemy` _asw_life_bar) (`KismetTextLibrary.Conv_StringToText` (`KismetStringLibrary.Concat_StrStr` (`KismetStringLibrary.Conv_IntToString` (`self.Hp`)) " / " (`KismetStringLibrary.Conv_IntToString` (`self.MaxHp`))))))

(fn `UserConstructionScript`)