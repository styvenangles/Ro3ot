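; Wave generator actor that spawns data-table-driven enemy waves and doubles as a typed spawn point, with a sprite per enemy type.
; SpawnWave sorts all generators by type, and BeginWave spawns the current row's enemies at random matching points.
; A one-second poll detects a cleared wave, increments the number and sets a countdown timer, though its zero time and no looping prevent counting.
; BeginPlay is empty and SpawnWave is unwired here.
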(event `self.ReceiveBeginPlay`)

(event `Spawn Enemy`
  (params (Class :type "Actor Class Reference") (SpawnTransform :type "Transform Structure") (NbEnemy :type Integer))
  (for _ (range NbEnemy)
    (bind _returnvalue (`|SpawnActorFromClass` Class SpawnTransform "AdjustIfPossibleButAlwaysSpawn" "OverrideRootScale" null null))
    (`KismetArrayLibrary.Array_Add` (`self.EnemyList`) _returnvalue))
  (`KismetSystemLibrary.Delay` (`self.Delay`))
  (`self.Spawn Enemy` (`self.Enemy`) (`self.GetTransform`) (`self.Last Index`)))

(event `SpawnWave`
  (bind _outactors (`GameplayStatics.GetAllActorsOfClass` "WaveGenerator_C"))
  (bind _output_get (set `self.Enemy Spawn` _outactors))
  (for _array_element _output_get
    (switch `/Game/Blueprint/EnemyWave/EnemyTypes` (`/Game/Blueprint/EnemyWave/WaveGenerator.EnemyType` _array_element)
      (:`NewEnumerator0`
        (`KismetArrayLibrary.Array_Add` (`self.LightEnemy`) _array_element))
      (:`NewEnumerator1`
        (`KismetArrayLibrary.Array_Add` (`self.NormalEnemy`) _array_element))
      (:`NewEnumerator2`
        (`KismetArrayLibrary.Array_Add` (`self.HeavyEnemy`) _array_element)))))

(event `Check Enemy Remaining`
  (bind _returnvalue (`KismetSystemLibrary.K2_SetTimerDelegate` (delegate `Count`)))
  (set `self.Timer` 3))

(event `Count`
  (`KismetSystemLibrary.PrintString` (`KismetStringLibrary.Conv_IntToString` (`self.Timer`)))
  (`/Engine/EditorBlueprintResources/StandardMacros.DecrementInt` (`self.Timer`)
    (:`  `
      (if (== (`self.Timer`) 0)
        (`KismetSystemLibrary.K2_ClearAndInvalidateTimerHandle` (stale `Check Enemy Remaining` _returnvalue))
        (`self.Begin Wave`)))))

(event `Begin Wave`
  (bind _returnvalue (`|GetDataTableRow` (`self.Data Table`) (`KismetStringLibrary.Conv_StringToName` (`KismetStringLibrary.Conv_IntToString` (`self.Wave Number`))))
    (:`then`
      (for _array_element (`.EnemyInfos_3_CCDBB8A34AA6F99637DAD082D14BE017` (break `/Game/Blueprint/EnemyWave/WaveInfo` _returnvalue))
        (`self.SpawnEnemy` _array_element))
      (`self.CheckIfEnemyDead`))))

(event `CheckIfEnemyDead`
  (bind _output_get (`self.CheckIfEnemiesAllDead` :!label _label))
  (if _output_get
    (`KismetSystemLibrary.PrintString` "All Enemies Dead")
    (`/Engine/EditorBlueprintResources/StandardMacros.IncrementInt` (`self.Wave Number`)
      (:`  `
        (`self.Check Enemy Remaining`)))
    (else
      (`KismetSystemLibrary.Delay` 1.0)
      (goto _label))))

(fn `CheckEnemy`)

(fn `CheckIfEnemiesAllDead`
  (returns (Output_Get :type Boolean))
  (locals (Dead :type Boolean))
  (set `local.Dead` true)
  (for _array_element (`self.Current Enemies`)
    (`/Engine/EditorBlueprintResources/StandardMacros.IsValid` _array_element
      (:`Is Valid`
        (set `local.Dead` false))))
  (return (`local.Dead`)))

(fn `SpawnEnemy`
  (params (EnemyInfo :type "/Game/Blueprint/EnemyWave/EnemyInfo Structure (by ref)"))
  (locals (`Current Spawn Point` :type "Array of /Game/Blueprint/EnemyWave/WaveGenerator Object Reference") (EnemyRef :type "/Game/Blueprint/EnemyWave/EnemyInfo Structure"))
  (bind _enemyref_enemyclass (break `/Game/Blueprint/EnemyWave/EnemyInfo` (`local.EnemyRef`)))
  (bind (_enemyref_enemyclass_2 _enemyref_enemynumber) (break `/Game/Blueprint/EnemyWave/EnemyInfo` (`local.EnemyRef`)))
  (bind _current_spawn_point (`local.Current Spawn Point`))
  (bind _output_get (set `local.EnemyRef` EnemyInfo))
  (set `local.Current Spawn Point` (select `/Game/Blueprint/EnemyWave/EnemyTypes` (`.EnemyType_8_47CF3B58473FCE0F3C51E28B77C626D7` (break `/Game/Blueprint/EnemyWave/EnemyInfo` _output_get)) :`NewEnumerator0` (`self.LightEnemy`) :`NewEnumerator1` (`self.NormalEnemy`) :`NewEnumerator2` (`self.HeavyEnemy`)))
  (for _ (range 1 (+ _enemyref_enemynumber 1))
    (bind _returnvalue (`|SpawnActorFromClass` _enemyref_enemyclass (`self.GetTransform` (`|GetArrayItem` _current_spawn_point (`KismetMathLibrary.RandomIntegerInRange` 0 (`KismetArrayLibrary.Array_LastIndex` _current_spawn_point)))) "AdjustIfPossibleButAlwaysSpawn" "OverrideRootScale" null null))
    (`KismetArrayLibrary.Array_Add` (`self.Current Enemies`) _returnvalue)))

(fn `UserConstructionScript`
  (`BillboardComponent.SetSprite` (`self.Target`) (select `/Game/Blueprint/EnemyWave/EnemyTypes` (`self.EnemyType`) :`NewEnumerator0` "/Game/Characters/Mannequins/Textures/Quinn/T_Quinn_01ID_D.T_Quinn_01ID_D" :`NewEnumerator1` "/Game/Characters/Mannequins/Textures/Quinn/T_Quinn_01ID_MSR_MSK.T_Quinn_01ID_MSR_MSK" :`NewEnumerator2` "/Game/Characters/Mannequins/Textures/Quinn/T_Quinn_02ID_D.T_Quinn_02ID_D" :!type "Texture2D Object Reference")))